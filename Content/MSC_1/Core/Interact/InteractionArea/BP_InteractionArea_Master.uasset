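; Master interaction area, used as a child actor, that handles focus and optional position restriction for its parent interactable.
; On BeginPlay it finds the parent's tagged restriction box and interaction widget.
; Focus changes notify the parent via interface message and toggle the widget, while CanFocus checks box overlap when a box exists.
; Box overlap events make the overlapping actor's BP_PlayerInteractionComponent reset its interaction trace.
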(event Custom|ToggleFocus
  (params (bFocused :type Boolean))
  (bind _interactwidgetcomponentref (Variables|Default|GetInteractWidgetComponentRef))
  ;[0.15 0.15 0.15 0.5] Toggle Highlight & Interaction Widget Visibility
  (Variables|Default|SetbFocused bFocused)
  (Class|BPIInteraction|InterfaceToggleFocus(Message) (Actor|GetParentActor) (Variables|Default|GetbFocused))
  (Utilities|IsValid _interactwidgetcomponentref
    (:Is%20Valid
      (Development|SetHiddeninGame _interactwidgetcomponentref (not (Variables|Default|GetbFocused)) false))))

(event Custom|OnComponentBeginOverlap_Event
  (params (OverlappedComponent :type Primitive%20Component%20Object%20Reference) (OtherActor :type Actor%20Object%20Reference) (OtherComp :type Primitive%20Component%20Object%20Reference) (OtherBodyIndex :type Integer) (bFromSweep :type Boolean) (SweepResult :type Hit%20Result%20Structure%20%28by%20ref%29))
  ;[0.15 0.15 0.15 0.5] Get Parent Actor Components
  ;;[0.15 0.15 0.15 0.5] Assign Parent Actor 'Restriction Box' Overlap Event Callbacks
  (CallFunction|ResetInteractionTrace OtherActor))

(event Custom|OnComponentEndOverlap_Event
  (params (OverlappedComponent :type Primitive%20Component%20Object%20Reference) (OtherActor :type Actor%20Object%20Reference) (OtherComp :type Primitive%20Component%20Object%20Reference) (OtherBodyIndex :type Integer))
  ;[0.15 0.15 0.15 0.5] Get Parent Actor Components
  ;;[0.15 0.15 0.15 0.5] Assign Parent Actor 'Restriction Box' Overlap Event Callbacks
  (CallFunction|ResetInteractionTrace OtherActor))

(event Custom|ResetInteractionTrace
  (params (Character :type Actor%20Object%20Reference))
  (bind _returnvalue (Actor|GetComponentbyClass Character "/Game/MSC_1/Core/Interact/PlayerInteract/BP_PlayerInteractionComponent.BP_PlayerInteractionComponent_C"))
  ;[0.15 0.15 0.15 0.5] Assign Parent Actor 'Restriction Box' Overlap Event Callbacks
  (Utilities|IsValid _returnvalue
    (:Is%20Valid
      (Default|ResetInteractionTrace _returnvalue))))

(event EventBeginPlay
  (bind _returnvalue (Actor|GetParentActor))
  (bind _returnvalue_2 (Actor|GetComponentsbyTag _returnvalue "/Script/Engine.ShapeComponent" "box"))
  (bind _output (Utilities|Array|Get(acopy) _returnvalue_2))
  ;[0.15 0.15 0.15 0.5] Get Parent Actor Components
  (Utilities|FlowControl|Sequence
    (:then_0
      ;;[0.15 0.15 0.15 0.5] Get 'Restriction Box'
      (Utilities|IsValid _output
        (:Is%20Valid
          (Variables|Default|SetbCharacterNeedsToBeInBox true)
          ;;[0.15 0.15 0.15 0.5] Assign Parent Actor 'Restriction Box' Overlap Event Callbacks
          (bind _output_get (Variables|Default|SetBoxRef _output))
          (Utilities|FlowControl|Sequence
            (:then_0
              (Collision|AssignOnComponentBeginOverlap _output_get (delegate Custom|OnComponentBeginOverlap_Event)))
            (:then_1
              (Collision|AssignOnComponentEndOverlap _output_get (delegate Custom|OnComponentEndOverlap_Event)))))))
    (:then_1
      ;;[0.15 0.15 0.15 0.5] Get Interaction Widget
      (Variables|Default|SetInteractWidgetComponentRef (Utilities|Array|Get(acopy) (Actor|GetComponentsbyTag (Actor|GetParentActor) "/Script/UMG.WidgetComponent" "Interact"))))))

(fn ConstructionScript)

(fn CanFocus
  (params (Character :type Actor%20Object%20Reference))
  (bind _boxref (Variables|Default|GetBoxRef))
  (Variables|Default|GetbCharacterNeedsToBeInBox
    (:then
      (Utilities|IsValid _boxref
        (:Is%20Valid
          (return (Collision|IsOverlappingActor _boxref Character :!class /Script/Engine.PrimitiveComponent)))))
    (:else
      (return true))))