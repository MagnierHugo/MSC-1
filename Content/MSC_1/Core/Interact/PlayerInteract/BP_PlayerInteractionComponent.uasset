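; Player component that lets the locally controlled pawn focus interaction areas and trigger them through IA_Interact.
; A looping timer runs camera line traces, toggling focus on BP_InteractionArea_Master actors that allow it.
; Interaction is instant or hold-based, with a second timer filling the area widget's round progress bar until completion, release or lost focus.
; Completion calls InteractOnServer, which sends an interface message with the pawn to the area's parent actor.
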(event Custom|EnableTrace
  ;[0.15 0.15 0.15 0.5] Start Trace Loop Timer
  (bind _returnvalue (Utilities|Time|SetTimerbyEvent (EventDispatchers|CreateEvent :!event Trace) (Variables|Trace|GetTimeBetweenTrace) true))
  (Variables|Trace|SetTimerHandle _returnvalue))

(event Custom|PauseTrace
  ;[0.15 0.15 0.15 0.5] Handle Trace
  (Utilities|Time|PauseTimerbyHandle (Variables|Trace|GetTimerHandle))
  (CallFunction|TraceInteractionArea false))

(event Custom|UnpauseTrace
  ;[0.15 0.15 0.15 0.5] Handle Trace
  (Utilities|Time|UnpauseTimerbyHandle (Variables|Trace|GetTimerHandle)))

(event Custom|StopTrace
  ;[0.15 0.15 0.15 0.5] Handle Trace
  (Utilities|Time|ClearandInvalidateTimerbyHandle (Variables|Trace|GetTimerHandle))
  (CallFunction|TraceInteractionArea false))

(event Custom|TryToInteract
  (params (In :type Boolean))
  ;[0.15 0.15 0.15 0.5] Try to interact with the focused actor
  (HeldObjects|Interaction|CanInteract In
    (:True
      (bind _output_get (Variables|Interaction|SetInteract%20Duration (Variables|/Game/MSC_1/Core/Interact/InteractionArea/BP_InteractionArea_Master.BP_InteractionArea_Master_C|GetInteractDuration (Variables|Trace|GetFocusedInteractionArea))))
      (if (> _output_get 0.0)
        (|GetCurrentInteractionWidgetProgressBarRef)
        (bind _returnvalue (Utilities|Time|SetTimerbyEvent (EventDispatchers|CreateEvent :!event Custom|UpdateInteractionProgress) (Variables|Interaction|GetUpdateInteractionInterval) true))
        (Variables|Interaction|SetInteractionTimerHandle _returnvalue)
        (else
          (CallFunction|InteractOnserver (Variables|Trace|GetFocusedInteractionArea))
          (CallFunction|RunEventAfterInteraction))))
    (:False
      (CallFunction|StopInteraction))))

(event Custom|InteractOnServer
  (params (InteractionArea :type BP%20Interaction%20Area%20Master%20Object%20Reference))
  ;[0.15 0.15 0.15 0.5] Dispatch interaction from server to clients
  (bind _aspawn (Utilities|Casting|CastToPawn (Components|GetOwner)))
  (Class|BPIInteraction|InterfaceInteract(Message) (Actor|GetParentActor InteractionArea) _aspawn))

(event Custom|UpdateInteractionProgress
  ;[0.15 0.15 0.15 0.5] Update Interaction timer & interaction widget progress bar
  (bind _output_get (Variables|Interaction|SetInteractionProgress (|({4F9CD930-42E5-C959-C6B5-E190D5550E65}+((1/InteractDuration)*{2F1E3147-4D1B-3329-D6A5-2CADF0A89371})) (Variables|Interaction|GetInteract%20Duration))))
  (Default|SetPercent (Variables|Interaction|GetCurrentInteractionWidgetProgressBarRef) _output_get)
  (if (>= (Variables|Interaction|GetInteractionProgress) 1.0)
    (CallFunction|StopInteraction)
    (CallFunction|InteractOnserver (Variables|Trace|GetFocusedInteractionArea))
    (CallFunction|RunEventAfterInteraction)))

(event Input|EnhancedActionEvents|EnhancedInputActionIA_Interact
  (params (ActionValue :type Boolean) (ElapsedSeconds :type Float%20%28double-precision%29) (TriggeredSeconds :type Float%20%28double-precision%29) (InputAction :type Input%20Action%20Object%20Reference :default "/Game/MSC_1/Core/Input/Actions/IA_Interact.IA_Interact"))
  ;[0.15 0.15 0.15 0.5] Interact Input Action
  (:Started
    (CallFunction|TrytoInteract true))
  (:Completed
    (CallFunction|TrytoInteract false)))

(event EventBeginPlay
  ;[0.15 0.15 0.15 0.5] Enable Trace only if the owner is the local player (multiplayer safe)
  (bind _aspawn (Utilities|Casting|CastToPawn (Components|GetOwner)))
  (if (Pawn|IsLocallyControlled _aspawn)
    (Utilities|FlowControl|Sequence
      (:then_0
        (CallFunction|EnableTrace))
      (:then_1
        (Class|BPIIMCHandling|AddIMC(Message) (Pawn|GetController _aspawn) "/Game/MSC_1/Core/Input/IMC_Interaction.IMC_Interaction")))))

(fn Trace
  (bind (_returnvalue _returnvalue2) (|GetTraceStartandEnd))
  (bind (_outhit _returnvalue_2) (Collision|LineTraceByChannel _returnvalue _returnvalue2 "TraceTypeQuery1" false 0 "None"))
  (if _returnvalue_2
    (Development|PrintString (Utilities|GetDisplayName (.HitActor (Collision|BreakHitResult _outhit))) true true "(R=1.000000,G=0.069560,B=0.858028,A=1.000000)" 2.0 "Interaction")
    (if (!= (Variables|Trace|GetFocusedActor) (.HitActor (Collision|BreakHitResult _outhit)))
      (Variables|Trace|SetFocusedActor (.HitActor (Collision|BreakHitResult _outhit)))
      (CallFunction|TraceInteractionArea (Utilities|ClassIsChildOf (Utilities|GetClass (.HitActor (Collision|BreakHitResult _outhit))) "/Game/MSC_1/Core/Interact/InteractionArea/BP_InteractionArea_Master.BP_InteractionArea_Master_C")))
    (else
      (CallFunction|TraceInteractionArea false))))

(fn TraceInteractionArea
  (params (bTrace :type Boolean))
  (if bTrace
    (if (Variables|Trace|GetbIsTracingInteractionArea)
      (Utilities|FlowControl|Sequence
        (:then_0
          (|UnfocusPreviousInteractionArea))
        (:then_1
          (|FocusInteractionArea :!label _label
            (:UnfocusTraced
              (if (Variables|Trace|GetbIsTracingInteractionArea) :!label _label_2
                (Variables|Trace|SetbIsTracingInteractionArea false)
                (Default|ToggleFocus (Variables|Trace|GetFocusedInteractionArea) false)
                (Variables|Trace|SetFocusedActor 0)
                (Variables|Trace|SetFocusedInteractionArea 0)
                (CallFunction|StopInteraction))))))
      (else
        (goto _label)))
    (else
      (goto _label_2))))

(fn StopInteraction
  (if (> (Variables|Interaction|GetInteractionProgress) 0.0)
    (Utilities|Time|ClearandInvalidateTimerbyHandle (Variables|Interaction|GetInteractionTimerHandle))
    (Default|SetPercent (Variables|Interaction|GetCurrentInteractionWidgetProgressBarRef) 0.0)
    (Variables|Interaction|SetInteractionProgress 0.0)
    (Variables|Interaction|SetCurrentInteractionWidgetProgressBarRef 0)))

(fn RunEventAfterInteraction)

(fn ResetInteractionTrace
  (CallFunction|TraceInteractionArea false))