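; BP_DemoInteractable is a demo interactable actor whose point light is switched on and off by player interaction.
; It implements BPI_Interaction, using custom depth on its cube to highlight it on focus.
; Interacting calls InteractOnServer, which flips InteractToggle, and that variable's RepNotify sets the light's visibility to replicate the state.
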(event Custom|InteractOnServer
  ;[0.15 0.15 0.15 0.5] BPI_Interaction Interface Implementation
  ;;[0.15 0.15 0.15 0.5] Server Replication
  (Variables|Default|SetInteractToggle (not (Variables|Default|GetInteractToggle))))

(event EventInterfaceInteract
  (params (Pawn :type Pawn%20Object%20Reference))
  ;[0.15 0.15 0.15 0.5] BPI_Interaction Interface Implementation
  ;;[0.15 0.15 0.15 0.5] Function Called on Player Interaction
  (CallFunction|InteractonServer))

(event EventInterfaceToggleFocus
  (params (Focus :type Boolean))
  ;[0.15 0.15 0.15 0.5] BPI_Interaction Interface Implementation
  ;;[0.15 0.15 0.15 0.5] Toggle Highlight on Mesh
  (Rendering|SetRenderCustomDepth (Variables|Default|GetCube) Focus))

(fn ConstructionScript)

(fn OnRepInteractToggle
  ;[0.15 0.15 0.15 0.5] Callback sent by the server on "InteractToggle" modification
  (Rendering|SetVisibility (Variables|Default|GetPointLight) (Variables|Default|GetInteractToggle) false))